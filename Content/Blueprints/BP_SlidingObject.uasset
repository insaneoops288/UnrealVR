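; BP_SlidingObject is a grabbable object that slides horizontally with the motion controller holding it.
; On grab, it checks that the controller is within the sphere's radius, then starts a looping quarter-second timer rather than using Tick.
; Each Slide call copies the controller's X and Y while keeping the Z height cached at BeginPlay.
; Dropping clears the controller and pauses the timer by function name.
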(event OnGrabbed(GrabComponent)
  (params (MotionController :type Motion%20Controller%20Component%20Object%20Reference))
  (bind _sphere (Variables|Default|GetSphere))
  (Utilities|IsValid MotionController
    (:Is%20Valid
      (bind _output_get (Variables|Default|SetMotion%20Controller MotionController))
      (if (Utilities|Operators|EqualEqual (Transformation|GetWorldLocation _output_get) (Transformation|GetWorldLocation _sphere) (Variables|/Script/Engine.SphereComponent|GetSphereRadius _sphere))
        ;[0.15 0.15 0.15 0.5] Time 0.25   Looping
        (Utilities|Time|SetTimerbyEvent (delegate Custom|Slide) 0.25 true)))))

(event OnDropped(GrabComponent)
  (Variables|Default|SetMotion%20Controller 0)
  ;[0.15 0.15 0.15 0.5] Slide Function Name
  (Class|KismetSystemLibrary|PauseTimer 0 "Slide"))

(event Custom|Slide
  (bind _motion_controller (Variables|Default|GetMotion%20Controller))
  (bind _returnvalue (Transformation|GetWorldLocation _motion_controller))
  (Transformation|SetWorldLocation (Variables|Default|GetSlidingObject) (Math|Vector|MakeVector (.x _returnvalue) (.y _returnvalue) (.z (Variables|Default|GetInitialLocation))) false false))

(event EventBeginPlay
  (Variables|Default|SetInitialLocation (Transformation|GetWorldLocation (Variables|Default|GetSlidingObject))))

(fn ConstructionScript)