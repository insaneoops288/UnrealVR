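; BP_RotatingObject is a grabbable object that turns about its pivot's up axis to follow a motion controller.
; When GrabComponent reports a grab with the controller inside the Sphere's radius, a looping quarter-second timer runs Rotate.
; Rotate keeps the pivot's up vector and aims its X axis directly away from the controller.
; Dropping clears the controller and pauses the timer; the initial rotation saved at BeginPlay is never applied.
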(event OnGrabbed(GrabComponent)
  (params (MotionController :type Motion%20Controller%20Component%20Object%20Reference))
  (bind _sphere (Variables|Default|GetSphere))
  (Utilities|IsValid MotionController
    (:Is%20Valid
      (bind _output_get (Variables|Default|SetMotion%20Controller MotionController))
      (if (Utilities|Operators|EqualEqual (Transformation|GetWorldLocation _output_get) (Transformation|GetWorldLocation _sphere) (Variables|/Script/Engine.SphereComponent|GetSphereRadius _sphere))
        ;[0.15 0.15 0.15 0.5] Time 0.25   Looping
        (Utilities|Time|SetTimerbyEvent (delegate Custom|Rotate) 0.25 true)))))

(event OnDropped(GrabComponent)
  (Variables|Default|SetMotion%20Controller 0)
  ;[0.15 0.15 0.15 0.5] Rotate Function Name
  (Class|KismetSystemLibrary|PauseTimer 0 "Rotate"))

(event Custom|Rotate
  (bind _rotatingobjectpivot (Variables|Default|GetRotatingObjectPivot))
  (Transformation|SetWorldRotation (Variables|Default|GetRotatingObjectPivot) (Math|Rotator|MakeRotfromZX (Math|Vector|GetUpVector _rotatingobjectpivot) (- (Transformation|GetWorldLocation _rotatingobjectpivot) (Transformation|GetWorldLocation (Variables|Default|GetMotion%20Controller)))) false false))

(event EventBeginPlay
  (Variables|Default|SetInitialRotation (Transformation|GetWorldRotation (Variables|Default|GetRotatingObjectPivot))))

(fn ConstructionScript)